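; Base unit Blueprint for selectable units that move on command and consume food over time.
; On BeginPlay it creates its own info widget, caches the HUD's info bar, and starts a looping timer that has the player controller subtract food.
; Selection toggles a decal and adds or removes that widget.
; It stores task info, and its move event uses AI MoveTo, resetting the task on success.
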(event Custom|SubtractFoodTimer
  ;[1 1 1] Subtract Food on Timer
  (Class|BPIInteraction|SubtractFood(Message) (Game|GetPlayerController 0) 15))

(event EventBeginPlay
  ;[1 1 1] Begin Play Setup
  (bind _ashud_ccb (Utilities|Casting|CastToHUD_CCB (HUD|GetHUD (Game|GetPlayerController 0))))
  (Variables|Default|SetUnit%20Info%20Bar%20Ref (Variables|/Game/Blueprints/Core/HUD_CCB.HUD_CCB_C|GetUnitInfoBarRef _ashud_ccb))
  (bind _returnvalue (UserInterface|CreateWidget "/Game/Widgets/WB_UnitInfo.WB_UnitInfo_C" 0 self))
  (Variables|Default|SetUnitInfoRef _returnvalue)
  (Utilities|Time|SetTimerbyFunctionName 0 "SubtractFoodTimer" 5.0 true))

(event EventUpdateTaskInfo
  (params (TaskInfo :type S%20Task%20Info%20Structure))
  ;[1 1 1] Update Task Info
  (Variables|Default|SetTaskInfo TaskInfo))

(event EventSelectUnit
  ;[1 1 1] Unit Selection/Deselection
  (Rendering|SetVisibility (Variables|Default|GetDecal) true false)
  (Class|BPIInteraction|AddChildtoInfoBar(Message) (Variables|Default|GetUnit%20Info%20Bar%20Ref) (Variables|Default|GetUnitInfoRef)))

(event EventDeselectUnit
  ;[1 1 1] Unit Selection/Deselection
  (Rendering|SetVisibility (Variables|Default|GetDecal) false false)
  (Widget|RemovefromParent (Variables|Default|GetUnitInfoRef)))

(event EventUnitMoveto
  (params (UnitRef :type BP%20Unit%20Base%20Object%20Reference) (Location :type Vector :default "0, 0, 0"))
  ;[1 1 1] Unit Move Command and TaskInfo Update
  (AI|AIMoveTo UnitRef Location 0 5.0 false
    (:OnSuccess
      (Variables|Default|SetTaskInfo (Utilities|Struct|MakeS_TaskInfo "NewEnumerator0" "NewEnumerator0" "0.000000,0.000000,0.000000")))))

(fn ConstructionScript)
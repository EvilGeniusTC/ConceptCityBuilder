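; PC_CCB is the player controller for an RTS-style game, handling marquee selection, unit move orders and the stored food total.
; It creates the main UI on BeginPlay and relays left-mouse press, hold and release to the HUD for selection.
; Right-click spaces destinations in a line along X from the hit location, then sets each selected unit's task and sends a move message.
; SubtractFood lowers the food total, printing a loss message at zero.
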(event EventTick
  (params (DeltaSeconds :type Float%20%28single-precision%29))
  ;[1 1 1] LMB // Marquee Selection
  (if (Variables|Default|GetIsPressedLMB)
    (Class|BPIInteraction|MarqueeHeld(Message) (HUD|GetHUD))))

(event EventBeginPlay
  ;[1 1 1] Begin Play Setup
  (Input|SetIgnoreLookInput false)
  (bind _returnvalue (Actor|GetActorOfClass "/Game/Blueprints/Core/HUD_CCB.HUD_CCB_C"))
  (Variables|Default|SetHUD%20Reference _returnvalue)
  (Input|SetInputModeGameandUI self 0 "LockAlways" false true)
  (bind _returnvalue_2 (UserInterface|CreateWidget "/Game/Widgets/WB_MainUI.WB_MainUI_C"))
  (bind _output_get (Variables|Default|SetMainUIRef _returnvalue_2))
  (UserInterface|Viewport|AddtoViewport _output_get 0))

(event EventSubtractFood
  (params (FoodToConsume :type Integer))
  ;[1 1 1] Consume Food
  (bind _output_get (Variables|Default|SetTotalFoodStored (Math|Integer|Clamp(Integer) (- (Variables|Default|GetTotalFoodStored) FoodToConsume) 0 1000000000)))
  (if (== _output_get 0)
    (Development|PrintString "YOU LOSE" true true "(R=0.000000,G=0.660000,B=1.000000,A=1.000000)" 1e+01)))

(event Input|MouseEvents|LeftMouseButton
  (params (Key :type Key%20Structure :default "None"))
  (bind _returnvalue (HUD|GetHUD))
  ;[1 1 1] LMB // Marquee Selection
  (:Pressed
    (Variables|Default|SetIsPressedLMB true)
    (Class|BPIInteraction|MarqueePressed(Message) _returnvalue))
  (:Released
    (Variables|Default|SetIsPressedLMB false)
    (Class|BPIInteraction|MarqueeReleased(Message) _returnvalue)))

(event Input|MouseEvents|RightMouseButton
  (params (Key :type Key%20Structure :default "None"))
  (bind _hud_reference (Variables|Default|GetHUD%20Reference))
  (bind _selectedunits (Variables|/Game/Blueprints/Core/HUD_CCB.HUD_CCB_C|GetSelectedUnits _hud_reference))
  ;[1 1 1] RMB // Unit Movement
  (:Pressed
    (Variables|Default|SetHitResultLocation (|HitResult))
    (for _array_element _selectedunits
      (Utilities|Array|Add (Variables|Default|GetHitResultLocations) (Variables|Default|GetHitResultLocation))
      (Variables|Default|SetHitResultLocation (+ (Variables|Default|GetHitResultLocation) "200.000000,0.000000,0.000000")))
    (for (_array_element_2 _array_index) _selectedunits
      (bind _asbp_unit_base (Utilities|Casting|CastToBP_Unit_Base _array_element_2))
      (bind _output_get (Variables|/Game/Blueprints/Units/BP_Unit_Base.BP_Unit_Base_C|SetTaskInfo _asbp_unit_base (Utilities|Struct|MakeS_TaskInfo "NewEnumerator1" "NewEnumerator1" (Utilities|Array|Get(acopy) (Variables|Default|GetHitResultLocations) _array_index))))
      (Class|BPIInteraction|UnitMoveto(Message) _asbp_unit_base _asbp_unit_base (.destination _output_get)))
    (Utilities|Array|Clear (Variables|Default|GetHitResultLocations))))

(fn ConstructionScript)
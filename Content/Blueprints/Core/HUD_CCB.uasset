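; HUD class that handles RTS-style unit selection by single pick or drag marquee and creates the unit info bar widget.
; Single selection clears all units via BPI_Interaction, selects one and tells Camera_CCB to look at it.
; While dragging, DrawHUD draws the rectangle and syncs SelectedUnits with GetSelectedActorsArray, sending select and deselect messages.
; That helper's BP_Unit_Base rectangle query appears unconnected.
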(event Custom|DeselectAll
  ;[1 1 1] Marquee Selection
  (bind _outactors (Actor|GetAllActorswithInterface "/Game/Interfaces/BPI_Interaction.BPI_Interaction_C"))
  (for _array_element _outactors
    (Class|BPIInteraction|DeselectUnit(Message) _array_element))
  (Utilities|Array|Clear (Variables|Default|GetSelectedUnits)))

(event EventBeginPlay
  ;[1 1 1] Begin Play Setup
  (bind _returnvalue (UserInterface|CreateWidget "/Game/Widgets/WB_UnitInfoBar.WB_UnitInfoBar_C"))
  (bind _output_get (Variables|Default|SetUnitInfoBarRef _returnvalue))
  (UserInterface|Viewport|AddtoViewport _output_get 0)
  (bind _returnvalue_2 (Actor|GetActorOfClass "/Game/Blueprints/Core/Camera_CCB.Camera_CCB_C"))
  (Variables|Default|SetCameraRef _returnvalue_2))

(event EventMarqueeReleased
  ;[1 1 1] Marquee Selection
  (Variables|Default|SetIsDrawing false))

(event EventMarqueePressed
  (bind _returnvalue (Game|GetPlayerController 0))
  (bind (_locationx _locationy) (Game|Player|GetMousePosition _returnvalue))
  ;[1 1 1] Marquee Selection
  (Utilities|FlowControl|Sequence
    (:then_0
      (CallFunction|DeselectAll))
    (:then_1
      (Variables|Default|SetIsDrawing true)
      (bind _output_get (Variables|Default|SetStartMousePosition (Math|Vector2D|MakeVector2D _locationx _locationy)))
      (Variables|Default|SetCurrentMousePosition _output_get))))

(event EventSelectSingleUnit
  (params (UnitRef :type Actor%20Object%20Reference))
  ;[1 1 1] Select Single Unit
  (CallFunction|DeselectAll)
  (Class|BPIInteraction|SelectUnit(Message) UnitRef)
  (Utilities|Array|Add (Variables|Default|GetSelectedUnits) UnitRef)
  (Class|BPIInteraction|LookatUnit(Message) (Variables|Default|GetCameraRef) UnitRef))

(event EventMarqueeHeld
  (bind _returnvalue (Game|GetPlayerController 0))
  (bind (_locationx _locationy) (Game|Player|GetMousePosition _returnvalue))
  ;[1 1 1] Marquee Selection
  (Variables|Default|SetCurrentMousePosition (Math|Vector2D|MakeVector2D _locationx _locationy)))

(event EventDrawHUD
  (params (SizeX :type Integer) (SizeY :type Integer))
  (bind _startmouseposition (Variables|Default|GetStartMousePosition))
  (bind _currentmouseposition (Variables|Default|GetCurrentMousePosition))
  ;[1 1 1] Marquee Selection
  (if (Variables|Default|GetIsDrawing)
    (HUD|DrawRect "(R=1.000000,G=0.000000,B=0.007402,A=0.277000)" (.x _startmouseposition) (.y _startmouseposition) (- (.x _currentmouseposition) (.x _startmouseposition)) (- (.y _currentmouseposition) (.y _startmouseposition)))
    (Variables|Default|SetActorsInRectangle (|GetSelectedActorsArray))
    (for _array_element (Variables|Default|GetActorsInRectangle)
      (Class|BPIInteraction|SelectUnit(Message) _array_element)
      (Utilities|Array|AddUnique (Variables|Default|GetSelectedUnits) _array_element))
    (for _array_element_2 (Variables|Default|GetSelectedUnits)
      (if (== (Utilities|Array|FindItem (Variables|Default|GetActorsInRectangle) _array_element_2) -1)
        (Class|BPIInteraction|DeselectUnit(Message) _array_element_2)
        (Utilities|Array|RemoveItem (Variables|Default|GetSelectedUnits) _array_element_2)))))

(fn ConstructionScript)